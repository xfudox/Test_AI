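; NPC sight test that changes the material color of SightTarget actors to show visibility.
; Every Tick it loops over all SightTargets, calls CheckForSight and changes or resets each one's color.
; CheckForSight compares the dot-product angle to PawnSensing's peripheral vision angle, then uses the controller's LineOfSightTo.
; As wired, neither the loop element reaches CheckForSight's Target nor any actor reaches LineOfSightTo.
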(event EventBeginPlay)

(event EventTick
  (params (DeltaSeconds :type Float%20%28single-precision%29))
  (bind _outactors (Actor|GetAllActorsOfClass "/Game/CommonAssets/SightTarget.SightTarget_C"))
  (bind _array_element (Utilities|Array|ForEachLoopwithBreak _outactors)
    (:LoopBody
      (bind _asnpc_character (Utilities|Casting|CastToNPC_Character self))
      (bind _result (CallFunction|CheckforSight _asnpc_character))
      (if _result
        (Default|ChangeMaterialColor _array_element)
        (else
          (Default|ResetMaterialColor _array_element))))))

(fn ConstructionScript)

(fn CheckforSight
  (params (Character :type NPC%20Character%20Object%20Reference%20%28by%20ref%29) (Target :type Actor%20Object%20Reference))
  (bind _returnvalue (Class|Actor|GetDotProductto Character Target))
  (bind _pawnsensing (Variables|/Game/NPC/Blueprints/NPC_Character.NPC_Character_C|GetPawnSensing Character))
  (bind _returnvalue_2 (Class|PawnSensingComponent|GetPeripheralVisionAngle _pawnsensing))
  (bind _returnvalue_3 (Class|KismetMathLibrary|DegAcos _returnvalue))
  (bind _returnvalue_4 (<= _returnvalue_3 _returnvalue_2))
  (if _returnvalue_4
    (return (Controller|LineOfSightTo (Pawn|GetController Character) 0 "0, 0, 0" false))
    (else
      (return _returnvalue_4))))