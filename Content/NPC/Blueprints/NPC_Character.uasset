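; NPC character Blueprint that spots members of other teams and switches between walking and running AI states.
; PawnSensing sightings of other NPC_Characters are compared by Team; an enemy's actor and location go to the Blackboard, and the NPC enters a running hide state.
; A wander event restores walk speed but is not called here.
; Construction sets speeds and tints the body material by team color; a StartAI call is left unconnected.
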(event OnSeePawn(PawnSensing)
  (params (Pawn :type Pawn%20Object%20Reference))
  (CallFunction|CheckforEnemy Pawn))

(event Custom|Set%20State%20To%20Hide
  (bind _output_get (Variables|Default|SetState "NewEnumerator2"))
  (AI|Components|Blackboard|SetValueasEnum (AI|GetBlackboard self) (Utilities|String|StringToName "State") _output_get)
  (Variables|/Script/Engine.CharacterMovementComponent|SetMaxWalkSpeed (Variables|Character|GetCharacterMovement) (Variables|Default|GetSpeed%20Run)))

(event Custom|Set%20State%20To%20Wander
  (bind _output_get (Variables|Default|SetState "NewEnumerator0"))
  (AI|Components|Blackboard|SetValueasEnum (AI|GetBlackboard self) (Utilities|String|StringToName "State") _output_get)
  (Variables|/Script/Engine.CharacterMovementComponent|SetMaxWalkSpeed (Variables|Character|GetCharacterMovement) (Variables|Default|GetSpeed%20Walk)))

(event Custom|CheckForEnemy
  (params (Pawn :type Pawn%20Object%20Reference))
  (bind _self self)
  (bind _teamcolor (Variables|Default|GetTeamColor))
  (bind _returnvalue (AI|GetBlackboard _self))
  (if (== (Utilities|GetClass Pawn) "NPC_Character_C")
    (bind _asnpc_character (Utilities|Casting|CastToNPC_Character Pawn)
      (:then
        (if (== (Variables|NPC_Character_C|GetTeam _asnpc_character) (Variables|Default|GetTeam self))
          (Development|PrintString "Seen buddy" true true _teamcolor)
          (else
            (Development|PrintString "Enemy spotted" true true _teamcolor)
            (AI|Components|Blackboard|SetValueasObject _returnvalue (Utilities|String|StringToName "Enemy Target") Pawn)
            (AI|Components|Blackboard|SetValueasVector _returnvalue (Utilities|String|StringToName "Enemy Last Location") (Transformation|GetActorLocation Pawn))
            (CallFunction|SetStatetoHide))))
      (:CastFailed
        (if true
          _)))))

(event EventBeginPlay)

(fn ConstructionScript
  (Variables|Default|SetSpeed%20Walk 2e+02)
  (Variables|Default|SetSpeed%20Run 6e+02)
  (Variables|/Script/Engine.CharacterMovementComponent|SetMaxWalkSpeed (Variables|Character|GetCharacterMovement) (Variables|Default|GetSpeed%20Walk))
  (bind _returnvalue (Rendering|Material|CreateDynamicMaterialInstance (Variables|Character|GetMesh) 0 "/Game/NPC/Character/Materials/M_UE4Man_Body.M_UE4Man_Body" :!class /Script/Engine.PrimitiveComponent))
  (Rendering|Material|SetVectorParameterValue _returnvalue "BodyColor" (Variables|Default|GetTeamColor) :!class /Script/Engine.MaterialInstanceDynamic))