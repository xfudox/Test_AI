(event OnSeePawn(PawnSensing)
  (params (Pawn :type Pawn%20Object%20Reference))
  (if (Utilities|ClassIsChildOf (Utilities|GetClass Pawn) "/Game/NPC/Blueprints/NPC_Main/NPC_Main.NPC_Main_C")
    _))

(event EventOnPossess
  (params (PossessedPawn :type Pawn%20Object%20Reference))
  (AI|RunBehaviorTree "/Game/NPC/AI/BehaviourTrees/BT_Main.BT_Main"))

(event EventBeginPlay
  (bind _output_get (Variables|Default|SetControlled%20Pawn (Pawn|GetControlledPawn)))
  (Variables|Default|SetControlled%20Pawn%20Blackboard (AI|GetBlackboard _output_get))
  (CallFunction|InitBlackboard))

(fn ConstructionScript
  (Development|PrintString (Utilities|GetDisplayName (Pawn|GetControlledPawn))))

(fn CheckLineOfSight
  (params (Target :type Actor%20Object%20Reference))
  (bind _pawnsensing (Variables|Default|GetPawnSensing))
  (if (<= (Transformation|GetDistanceTo Target) (Variables|/Script/AIModule.PawnSensingComponent|GetSightRadius _pawnsensing))
    (if (<= (Class|KismetMathLibrary|DegAcos (Class|Actor|GetDotProductto Target)) (Class|PawnSensingComponent|GetPeripheralVisionAngle _pawnsensing))
      ;[1 1 1] Ostruito o no
      (return (Controller|LineOfSightTo Target "0, 0, 0" false))
      (else
        ;[1 1 1] Fuori cono visivo
        (return false)))
    (else
      ;[1 1 1] Fuori portata
      (return false))))

(fn SetPatrolData
  (params (NewParam :type Array%20of%20Vectors))
  ;[1 1 1] Store patrol waypoints
  (bind _output_get (Variables|Default|SetPatrolRouteWaypoints NewParam)))

(fn InitBlackboard
  (params (Possessed%20Pawn :type Pawn%20Object%20Reference))
  (bind _controlled_pawn_blackboard (Variables|Default|GetControlled%20Pawn%20Blackboard))
  (Class|BlackboardComponent|SetValueasInt _controlled_pawn_blackboard (Utilities|String|StringToName "Nex Patrol Waypoint"))
  (Class|BlackboardComponent|SetValueasInt _controlled_pawn_blackboard (Utilities|String|StringToName "Total Patrol Waypoints")))