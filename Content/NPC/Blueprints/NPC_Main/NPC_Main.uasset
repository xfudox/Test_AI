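; NPC_Main is an NPC character Blueprint with walk and run speeds, a sight check and a physics-based death.
; Construction sets both speed values and applies walk speed to CharacterMovement.
; CheckLineOfSight manually tests a target against PawnSensing's radius and peripheral cone, then the controller's LineOfSightTo for obstruction.
; Die enables physics simulation on mesh and capsule, while BeginPlay and SetBalloon are empty.
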(event EventBeginPlay)

(fn ConstructionScript
  (Variables|Default|SetSpeed%20Walk 2e+02)
  (Variables|Default|SetSpeed%20Run 6e+02)
  (Variables|/Script/Engine.CharacterMovementComponent|SetMaxWalkSpeed (Variables|Character|GetCharacterMovement) (Variables|Default|GetSpeed%20Walk)))

(fn CheckLineOfSight
  (params (Target :type Actor%20Object%20Reference))
  (if (<= (Transformation|GetDistanceTo Target) (Variables|/Script/AIModule.PawnSensingComponent|GetSightRadius (Variables|Default|GetPawnSensing)))
    (if (<= (Class|KismetMathLibrary|DegAcos (Class|Actor|GetDotProductto Target)) (Class|PawnSensingComponent|GetPeripheralVisionAngle (Variables|Default|GetPawnSensing)))
      ;[1 1 1] Ostruito o no
      (return (Controller|LineOfSightTo (Pawn|GetController) Target "0, 0, 0" false))
      (else
        ;[1 1 1] Fuori cono visivo
        (return false)))
    (else
      ;[1 1 1] Fuori portata
      (return false))))

(fn Die
  (Physics|SetSimulatePhysics (Variables|Character|GetMesh) true))

(fn SetBalloon
  (params (BalloonState :type Enum_Balloons%20Enum)))